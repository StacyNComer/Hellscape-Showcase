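; Test enemy Blueprint that serves as a debug target for inspecting incoming damage.
; Its DamageFeedback event prints damage dealt, remaining health, attack potency and damage type on screen in colored text.
; The OnTakeDamage binding for that event and a stun message check are disconnected, so neither runs.
; Tick only calls the parent, and BeginPlay and construction are empty.
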(event Custom|Damage%20Feedback
  (params (damageData :type Damage%20Data%20Object%20Reference) (attackDamageType :type Attack%20Damage%20Type%20Object%20Reference) (attackData :type Attack%20Data%20Structure))
  (Development|PrintString (Utilities|String|Append "Damage Dealt: " (Utilities|String|ToString(Float) (Variables|/Script/Hellscape.DamageData|Getdamage damageData))) true true "(R=0.000000,G=1.000000,B=0.291096,A=1.000000)")
  (Development|PrintString (Utilities|String|Append "Remaining Health: " (Utilities|String|ToString(Float) (Variables|Default|GetcurrentHealth))) true true "(R=1.000000,G=0.504662,B=0.000000,A=1.000000)")
  (Development|PrintString (Utilities|String|Append "Attack Potency: " (Utilities|String|ToString(Float) (Variables|/Script/Hellscape.DamageData|Getpotency damageData))) true true "(R=0.462804,G=0.000000,B=1.000000,A=1.000000)")
  (Development|PrintString (Utilities|String|EnumtoString (Variables|/Script/Hellscape.AttackDamageType|GetdamageType attackDamageType)) true true "(R=1.000000,G=0.504662,B=0.000000,A=1.000000)"))

(event EventBeginPlay)

(event Collision|EventActorBeginOverlap
  (params (OtherActor :type Actor%20Object%20Reference)))

(event EventTick
  (params (DeltaSeconds :type Float%20%28single-precision%29))
  (|CallParentFunction DeltaSeconds))

(fn ConstructionScript)