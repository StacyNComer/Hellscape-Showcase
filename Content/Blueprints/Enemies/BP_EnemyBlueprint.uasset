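; Enemy Blueprint that shows floating damage numbers as Niagara particles.
; SpawnDamageParticles splits the damage value into digits and spawns one NS_DamageNumbers system per digit on ParticleSpawn, spacing them sideways around the center.
; Each system receives the text color and a matching digit texture through user parameters.
; Tick rotates ParticleSpawn to follow the first player's control yaw so the numbers stay oriented to the view.
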(event EventBeginPlay)

(event Collision|EventActorBeginOverlap
  (params (OtherActor :type Actor%20Object%20Reference)))

(event EventTick
  (params (DeltaSeconds :type Float%20%28single-precision%29))
  (Transformation|SetWorldRotation (Variables|Default|GetParticle%20Spawn) (Math|Rotator|MakeRotator 0.0 1.8e+02 (.yaw (Pawn|GetControlRotation (Game|GetPlayerController 0) :!class /Script/Engine.Controller))) false false))

(event EventSpawnDamageParticles
  (params (damage :type Integer) (textColor :type Linear%20Color%20Structure))
  (CallFunction|DamageParticleFunction damage textColor))

(fn ConstructionScript)

(fn DamageParticleFunction
  (params (Damage :type Integer) (Text%20Color :type Linear%20Color%20Structure))
  (bind _returnvalue (Utilities|String|ToString(Integer) Damage))
  (bind _returnvalue_2 (Utilities|String|GetCharacterArrayfromString _returnvalue))
  (LocalVariables|SetText%20Offset (Math|Conversions|ToFloat(Integer) (* (- (Utilities|Array|Length _returnvalue_2) 1) -15)))
  (for _array_element _returnvalue_2
    (bind _returnvalue_3 (Niagara|SpawnSystemAttached "/Game/_Graphics/Particles/NS_DamageNumbers.NS_DamageNumbers" (Variables|Default|GetParticle%20Spawn) "None" "0, 0, 0" (Math|Rotator|MakeRotator 0.0 0.0 0.0) "KeepRelativeOffset" false))
    (bind _output_get (LocalVariables|SetDigit%20System _returnvalue_3))
    (Transformation|AddLocalOffset _output_get (Math|Vector|MakeVector 0.0 (LocalVariables|GetText%20Offset) 0.0) false false)
    (LocalVariables|SetText%20Offset (+ (LocalVariables|GetText%20Offset) 3e+01))
    (Niagara|SetNiagaraVariable(LinearColor) (LocalVariables|GetDigit%20System) "user.Color" Text%20Color)
    (switch string _array_element
      (:0
        (Niagara|SetTextureObject (LocalVariables|GetDigit%20System) "user.Digit" "/Game/_Graphics/Textures/numberTextures/0.0"))
      (:1
        (Niagara|SetTextureObject (LocalVariables|GetDigit%20System) "user.Digit" "/Game/_Graphics/Textures/numberTextures/1.1"))
      (:2
        (Niagara|SetTextureObject (LocalVariables|GetDigit%20System) "user.Digit" "/Game/_Graphics/Textures/numberTextures/2.2"))
      (:3
        (Niagara|SetTextureObject (LocalVariables|GetDigit%20System) "user.Digit" "/Game/_Graphics/Textures/numberTextures/3.3"))
      (:4
        (Niagara|SetTextureObject (LocalVariables|GetDigit%20System) "user.Digit" "/Game/_Graphics/Textures/numberTextures/4.4"))
      (:5
        (Niagara|SetTextureObject (LocalVariables|GetDigit%20System) "user.Digit" "/Game/_Graphics/Textures/numberTextures/5.5"))
      (:6
        (Niagara|SetTextureObject (LocalVariables|GetDigit%20System) "user.Digit" "/Game/_Graphics/Textures/numberTextures/6.6"))
      (:7
        (Niagara|SetTextureObject (LocalVariables|GetDigit%20System) "user.Digit" "/Game/_Graphics/Textures/numberTextures/7.7"))
      (:8
        (Niagara|SetTextureObject (LocalVariables|GetDigit%20System) "user.Digit" "/Game/_Graphics/Textures/numberTextures/8.8"))
      (:9
        (Niagara|SetTextureObject (LocalVariables|GetDigit%20System) "user.Digit" "/Game/_Graphics/Textures/numberTextures/9.9")))))