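; Enemy character Blueprint that handles death, damage feedback and dash collisions, mostly with debug output.
; On BeginPlay it caches the original walk speed and binds a take-damage handler that prints damage dealt and remaining health.
; Hits on a player character while dashing only print a message, and Die destroys the actor.
; The damage particle event and construction script are empty.
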(event Custom|Damage%20Feedback
  (params (damageData :type Damage%20Data%20Object%20Reference) (attackDamageType :type Attack%20Damage%20Type%20Object%20Reference) (attackData :type Attack%20Data%20Structure))
  (Development|PrintString (Utilities|String|Append "Damage Dealt: " (Utilities|String|ToString(Float) (Variables|/Script/Hellscape.DamageData|Getdamage damageData))) true true "(R=0.000000,G=1.000000,B=0.291096,A=1.000000)")
  (Development|PrintString (Utilities|String|Append "Remaining Health: " (Utilities|String|ToString(Float) (Variables|Default|GetcurrentHealth))) true true "(R=1.000000,G=0.504662,B=0.000000,A=1.000000)"))

(event EventBeginPlay
  (Variables|Default|SetOriginal%20Walk%20Speed (Variables|/Script/Engine.CharacterMovementComponent|GetMaxWalkSpeed (Variables|Character|GetCharacterMovement)))
  (EventDispatchers|AssignOnTakeDamage (delegate Custom|Damage%20Feedback)))

(event EventSpawnDamageParticles
  (params (damage :type Integer)))

(event Collision|EventHit
  (params (MyComp :type Primitive%20Component%20Object%20Reference) (Other :type Actor%20Object%20Reference) (OtherComp :type Primitive%20Component%20Object%20Reference) (bSelfMoved :type Boolean) (HitLocation :type Vector :default "0, 0, 0") (HitNormal :type Vector :default "0, 0, 0") (NormalImpulse :type Vector :default "0, 0, 0") (Hit :type Hit%20Result%20Structure%20%28by%20ref%29))
  (if (Variables|Default|GetIsDashing)
    (Utilities|Casting|CastToPlayerCharacterBase Other)
    (Development|PrintString "Gotyem!")))

(event EventDie
  (Actor|DestroyActor))

(fn ConstructionScript)