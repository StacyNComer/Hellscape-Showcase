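; BP_Laser is a castable focus item that fires a hitscan laser and damages enemies.
; Cast runs the parent logic, then line traces forward from the projectile spawn point on the Camera channel, with debug drawing enabled.
; A Niagara beam ends at the hit point or maximum range, tinted by the damage type's color.
; Enemy hits apply modified damage and potency, with critical multipliers for the Head bone.
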(event EventCast
  (bind _returnvalue (Transformation|GetActorForwardVector))
  (bind _projectilespawnpoint (Variables|Default|GetProjectileSpawnPoint))
  (bind _damage (Variables|Default|Getdamage))
  (bind _potency (Variables|Default|Getpotency))
  (bind _projectilespawnpoint_2 (Variables|Default|GetProjectileSpawnPoint))
  (bind _returnvalue_2 (Transformation|GetWorldTransform _projectilespawnpoint_2))
  (bind _returnvalue_3 (Transformation|GetWorldLocation _projectilespawnpoint))
  (bind _returnvalue_4 (* _returnvalue 5e+03))
  (bind _returnvalue_5 (+ _returnvalue_3 _returnvalue_4))
  (|CallParentFunction)
  (bind (_outhit _returnvalue_6) (Collision|LineTraceByChannel _returnvalue_3 _returnvalue_5 "TraceTypeQuery2" false 0 "ForDuration" true "(R=1.000000,G=0.000000,B=0.000000,A=1.000000)" "(R=0.000000,G=1.000000,B=0.000000,A=1.000000)" 0.0))
  (bind _returnvalue_7 (Niagara|SpawnSystematLocation "/Game/_Graphics/Particles/NS_Laser.NS_Laser" (.location _returnvalue_2) (.rotation _returnvalue_2)))
  (Niagara|SetNiagaraVariable(Vector3) _returnvalue_7 "BeamEndPoint" (select _returnvalue_6 (.location _outhit) _returnvalue_5))
  (Niagara|SetNiagaraVariable(LinearColor) _returnvalue_7 "Color" (Variables|/Script/Hellscape.AttackDamageType|Getcolor (Variables|Default|GetattackDamageType)))
  (bind _asenemy_base (Utilities|Casting|CastToEnemyBase (.hitactor _outhit)))
  (Class|EnemyBase|DamageEnemy _asenemy_base (Math|Float|SelectFloat (* (.modified _damage) (.modified (Variables|Default|GetcritDamageMultiplier))) (.modified _damage) (Utilities|Name|Equal(Name) (.hitbonename _outhit) "Head")) (Math|Float|SelectFloat (* (.modified _potency) (.modified (Variables|Default|GetcritPotencyMultiplier))) (.modified _potency) (Utilities|Name|Equal(Name) (.hitbonename _outhit) "Head")) (Variables|Default|GetattackDamageType) (Utilities|Struct|MakeAttackData (Variables|Default|GetwieldingPlayer) self false (Utilities|Name|Equal(Name) (.hitbonename _outhit) "Head") false)))

(fn ConstructionScript
  (|CallParentFunction))