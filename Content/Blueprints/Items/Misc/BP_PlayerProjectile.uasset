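; Base-style player projectile that damages EnemyBase actors it overlaps, then destroys itself.
; On overlap it records the enemy as the excluded actor and passes damage, potency, damage type and attack data to DamageEnemy.
; Any hit event also destroys it, while other overlapping actors are ignored.
; A helper function creates a dynamic material instance on a given mesh and tints it with the damage type's color.
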(event Collision|EventHit
  (params (MyComp :type Primitive%20Component%20Object%20Reference) (Other :type Actor%20Object%20Reference) (OtherComp :type Primitive%20Component%20Object%20Reference) (bSelfMoved :type Boolean) (HitLocation :type Vector :default "0, 0, 0") (HitNormal :type Vector :default "0, 0, 0") (NormalImpulse :type Vector :default "0, 0, 0") (Hit :type Hit%20Result%20Structure%20%28by%20ref%29))
  (Actor|DestroyActor))

(event Collision|EventActorBeginOverlap
  (params (OtherActor :type Actor%20Object%20Reference))
  (bind _asenemy_base (Utilities|Casting|CastToEnemyBase OtherActor))
  (Variables|Default|SetExcluded%20Actor _asenemy_base)
  (Class|EnemyBase|DamageEnemy _asenemy_base (Variables|Default|GetDamage) (Variables|Default|GetPotency) (Variables|Default|GetAttack%20Damage%20Type) (Variables|Default|GetDamage%20Data))
  (Actor|DestroyActor))

(fn ConstructionScript
  (Components|Movement|SetUpdatedComponent (Variables|Default|GetProjectileMovement) 0))

(fn InitializeProjectileMesh
  (params (Mesh%20Component :type Mesh%20Component%20Object%20Reference) (Material%20Index :type Integer) (Dynamic%20Material :type Material%20Interface%20Object%20Reference))
  (bind _returnvalue (Rendering|Material|CreateDynamicMaterialInstance Mesh%20Component Material%20Index Dynamic%20Material "None" :!class /Script/Engine.PrimitiveComponent))
  (Rendering|Material|SetVectorParameterValue _returnvalue "Color" (Variables|/Script/Hellscape.AttackDamageType|Getcolor (Variables|Default|GetAttack%20Damage%20Type)) :!class /Script/Engine.MaterialInstanceDynamic))