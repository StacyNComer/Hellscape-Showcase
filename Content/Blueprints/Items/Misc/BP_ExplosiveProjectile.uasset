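; Explosive projectile, a child of a base projectile, that detonates whenever it is destroyed.
; On Destroyed it spawns a BP_DamageArea with fixed damage and potency, passing along its attack type, damage data and excluded actor.
; A placeholder Niagara explosion is sized from the damage area's radius and tinted by the attack type's color.
; The construction script extends the parent's, initializing the sphere mesh with a dynamic color material.
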(event EventDestroyed
  (bind _returnvalue (Game|SpawnActorfromClass "/Game/Blueprints/Items/Misc/BP_DamageArea.BP_DamageArea_C" (Math|Transform|MakeTransform (Transformation|GetActorLocation) (Transformation|GetActorRotation) "1,1,1") "Undefined" 0 5e+01 2e+01 (Variables|Default|GetAttack%20Damage%20Type) (Variables|Default|GetDamage%20Data) (Variables|Default|GetExcluded%20Actor) 0))
  (bind _returnvalue_2 (Niagara|SpawnSystematLocation "/Game/_Graphics/Particles/NS_ExplosionPlaceholder.NS_ExplosionPlaceholder" (Transformation|GetActorLocation)))
  (Niagara|SetNiagaraVariable(Float) _returnvalue_2 "Size" (* (Default|GetAreaRadius _returnvalue) 2.0))
  (Niagara|SetNiagaraVariable(LinearColor) _returnvalue_2 "Color" (Variables|/Script/Hellscape.AttackDamageType|Getcolor (Variables|Default|GetAttack%20Damage%20Type))))

(fn ConstructionScript
  (|CallParentFunction)
  (CallFunction|InitializeProjectileMesh (Variables|Default|GetSphere) 0 "/Game/_Graphics/Materials/M_DynamicColor.M_DynamicColor"))