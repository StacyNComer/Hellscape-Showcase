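; BP_DamageArea is a one-shot spherical area-of-effect actor that damages the enemies inside it.
; On its first Tick it calls DamageEnemy on every overlapping EnemyBase except ExcludedActor, passing its damage, potency, attack type and attack data, then destroys itself.
; GetAreaRadius exposes the radius of its Sphere component.
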(event EventTick
  (params (DeltaSeconds :type Float%20%28single-precision%29))
  (for _array_element (Collision|GetOverlappingActors "/Script/Hellscape.EnemyBase" :!class /Script/Engine.Actor)
    (if (!= _array_element (Variables|Default|GetExcluded%20Actor))
      (bind _asenemy_base (Utilities|Casting|CastToEnemyBase _array_element))
      (Class|EnemyBase|DamageEnemy _asenemy_base (Variables|Default|GetDamage) (Variables|Default|GetPotency) (Variables|Default|GetAttack%20Type) (Variables|Default|GetAttack%20Data))))
  (Actor|DestroyActor))

(fn ConstructionScript)

(fn GetAreaRadius
  (return (Variables|/Script/Engine.SphereComponent|GetSphereRadius (Variables|Default|GetSphere))))